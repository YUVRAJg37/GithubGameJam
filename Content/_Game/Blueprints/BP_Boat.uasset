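; Drivable boat pawn that the player character can board and leave with Interact.
; A sphere overlap binds the player's interact event and shows a prompt widget; taking control possesses the boat and attaches the player at Steering.
; Possession swaps hand over the spring arm's world transform, then ease it to its default for smooth camera transitions.
; Physics on the Box drives movement: torque steers and force gives forward-only thrust, with no reverse.
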(event OnComponentBeginOverlap(Sphere)
  (params (OverlappedComponent :type Primitive%20Component%20Object%20Reference) (OtherActor :type Actor%20Object%20Reference) (OtherComp :type Primitive%20Component%20Object%20Reference) (OtherBodyIndex :type Integer) (bFromSweep :type Boolean) (SweepResult :type Hit%20Result%20Structure%20%28by%20ref%29))
  (bind _asplayer_character_bp (Utilities|Casting|CastToPlayerCharacter_BP OtherActor))
  (bind _output_get (Variables|Default|SetPlayer _asplayer_character_bp))
  (EventDispatchers|BindEventtoInteract _output_get (delegate Custom|TakeControlOfBoat))
  (if (not (Variables|Default|GetInteractSet))
    (Variables|Default|SetInteractSet true)
    (bind _returnvalue (UserInterface|CreateWidget "/Game/_Game/UI/UI_Equip.UI_Equip_C" (Game|GetPlayerController 0)))
    (bind _output_get_2 (Variables|Default|SetHud _returnvalue))
    (UserInterface|Viewport|AddtoPlayerScreen _output_get_2)))

(event OnComponentEndOverlap(Sphere)
  (params (OverlappedComponent :type Primitive%20Component%20Object%20Reference) (OtherActor :type Actor%20Object%20Reference) (OtherComp :type Primitive%20Component%20Object%20Reference) (OtherBodyIndex :type Integer))
  (bind _asplayer_character_bp (Utilities|Casting|CastToPlayerCharacter_BP OtherActor))
  (EventDispatchers|UnbindallEventsfromInteract _asplayer_character_bp)
  (if (Variables|Default|GetInteractSet)
    (Widget|RemovefromParent (Variables|Default|GetHud))
    (Variables|Default|SetInteractSet false)))

(event Custom|TakeControlOfBoat
  (bind _cameradefaulttransform (Variables|Default|GetCameraDefaultTransform))
  (bind _player (Variables|Default|GetPlayer))
  (bind _steering (Variables|Default|GetSteering))
  (Variables|Default|SetPlayerDefaultTransform (Transformation|GetRelativeTransform (Variables|/Game/_Game/Blueprints/PlayerCharacter/PlayerCharacter_BP.PlayerCharacter_BP_C|GetSpringArm (stale OnComponentBeginOverlap(Sphere) _output_get))))
  (Transformation|SetWorldTransform (Variables|Default|GetSpringArm) (Transformation|GetWorldTransform (Variables|/Game/_Game/Blueprints/PlayerCharacter/PlayerCharacter_BP.PlayerCharacter_BP_C|GetSpringArm (stale OnComponentBeginOverlap(Sphere) _output_get))) false false)
  (Pawn|Possess (Game|GetPlayerController 0) self)
  (Widget|RemovefromParent (Variables|Default|GetHud))
  (Variables|Default|SetInteractSet false)
  (Collision|SetActorEnableCollision _player false)
  (Transformation|SetActorLocation _player (Transformation|GetWorldLocation _steering) false false)
  (Transformation|AttachComponentToComponent _player _steering "None" "KeepWorld" "KeepRelative" "KeepWorld" false)
  (Components|MoveComponentTo (Variables|Default|GetSpringArm) (.location _cameradefaulttransform) (.rotation _cameradefaulttransform) false true 0.5 false))

(event EventBeginPlay
  (Variables|Default|SetCameraDefaultTransform (Transformation|GetRelativeTransform (Variables|Default|GetSpringArm))))

(event EventTick
  (params (DeltaSeconds :type Float%20%28single-precision%29)))

(event Input|ActionEvents|InputActionInteract
  (params (Key :type Key%20Structure :default "None"))
  (bind _playerdefaulttransform (Variables|Default|GetPlayerDefaultTransform))
  (bind _player (Variables|Default|GetPlayer))
  (bind _springarm (Variables|/Game/_Game/Blueprints/PlayerCharacter/PlayerCharacter_BP.PlayerCharacter_BP_C|GetSpringArm _player))
  (:Pressed
    (Utilities|IsValid _player
      (:Is%20Valid
        (Pawn|Possess (Game|GetPlayerController 0) _player)
        (Collision|SetActorEnableCollision _player true)
        (Transformation|SetWorldTransform _springarm (Transformation|GetWorldTransform (Variables|Default|GetSpringArm)) false false)
        (Components|MoveComponentTo _springarm (.location _playerdefaulttransform) (.rotation _playerdefaulttransform) true false 0.2 true)))))

(event Input|AxisEvents|InputAxisSteer
  (params (AxisValue :type Float%20%28single-precision%29))
  (if (!= AxisValue 0.0)
    (Class|PrimitiveComponent|AddTorqueinRadians (Variables|Default|GetBox) (Math|Vector|MakeVector 0.0 0.0 (* (Variables|Default|GetSteeringSensitivity) AxisValue)) "None" true)))

(event Input|AxisEvents|InputAxisMoveForward/Backward
  (params (AxisValue :type Float%20%28single-precision%29))
  (bind _box (Variables|Default|GetBox))
  (Math|Float|CompareFloat AxisValue 0.0
    (:>
      (Class|PrimitiveComponent|AddForceatLocation _box (* (Math|Vector|GetForwardVector _box) (Variables|Default|GetBoatSpeed) 1e+04) (Transformation|GetWorldLocation (Variables|Default|GetBox)) "None"))))

(fn ConstructionScript)