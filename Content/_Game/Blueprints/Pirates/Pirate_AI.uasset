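; Pirate_AI is the AI controller for pirate enemies, sending them after the player to attack.
; On BeginPlay it caches the controlled pirate and player character and starts a looping timer that calls Follow Player every few seconds after an initial delay.
; Each call issues an AI MoveTo toward the player; on success it briefly sets the pirate's Attacking flag, then clears it.
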(event Custom|Follow%20Player
  (bind _as_pirate_bp (Variables|Default|GetAs%20Pirate%20BP))
  (AI|AIMoveTo (Variables|Default|GetAs%20Pirate%20BP) "0, 0, 0" (Variables|Default|GetAs%20Player%20Character%20BP) 5.0 true
    (:OnSuccess
      (Variables|/Game/_Game/Blueprints/Pirates/Pirate_BP.Pirate_BP_C|SetAttacking _as_pirate_bp true)
      (Utilities|FlowControl|Delay 1.0)
      (Variables|/Game/_Game/Blueprints/Pirates/Pirate_BP.Pirate_BP_C|SetAttacking _as_pirate_bp false))))

(event EventBeginPlay
  (Utilities|Time|SetTimerbyFunctionName 0 "Follow Player" 3.0 true 1e+01)
  (bind _aspirate_bp (Utilities|Casting|CastToPirate_BP (Pawn|GetControlledPawn)))
  (Variables|Default|SetAs%20Pirate%20BP _aspirate_bp)
  (bind _asplayer_character_bp (Utilities|Casting|CastToPlayerCharacter_BP (Game|GetPlayerCharacter 0)))
  (Variables|Default|SetAs%20Player%20Character%20BP _asplayer_character_bp))

(event EventTick
  (params (DeltaSeconds :type Float%20%28single-precision%29)))

(fn ConstructionScript)