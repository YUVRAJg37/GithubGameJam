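; Pirate actor that takes damage, dies and can hurt the player.
; Incoming damage lowers its health, spawns an explosion effect and grants brief immunity through a delay-reset flag.
; Tick polls health and, at zero or below, spawns a larger explosion and destroys the actor.
; While the Attacking flag is set, overlaps on HitCollider apply Strength-based damage to actors tagged Player.
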(event OnComponentBeginOverlap(HitCollider)
  (params (OverlappedComponent :type Primitive%20Component%20Object%20Reference) (OtherActor :type Actor%20Object%20Reference) (OtherComp :type Primitive%20Component%20Object%20Reference) (OtherBodyIndex :type Integer) (bFromSweep :type Boolean) (SweepResult :type Hit%20Result%20Structure%20%28by%20ref%29))
  ;[1 1 1] Hitting Player
  (if (Variables|Default|GetAttacking)
    (if (Actor|ActorHasTag OtherActor "Player")
      (Game|Damage|ApplyDamage OtherActor (Math|Conversions|ToFloat(Integer) (Variables|Default|GetStrength)) 0 0))))

(event EventBeginPlay)

(event Collision|EventActorBeginOverlap
  (params (OtherActor :type Actor%20Object%20Reference)))

(event EventTick
  (params (DeltaSeconds :type Float%20%28single-precision%29))
  ;[1 1 1] Pirate Death
  (bind _output_get (Variables|Default|SetDead (<= (Variables|Default|GetPirateHealth) 0.0)))
  (if _output_get
    (Development|PrintString "Dead")
    (Effects|SpawnEmitteratLocation "/Game/StarterContent/Particles/P_Explosion.P_Explosion" (Transformation|GetActorLocation) "0, 0, 0" "3.000000,3.000000,3.000000")
    (Actor|DestroyActor)))

(event Game|Damage|EventAnyDamage
  (params (Damage :type Float%20%28single-precision%29) (DamageType :type Damage%20Type%20Object%20Reference) (InstigatedBy :type Controller%20Object%20Reference) (DamageCauser :type Actor%20Object%20Reference))
  ;[1 1 1] Getting Damage
  (if (not (Variables|Default|GetImmune))
    (Variables|Default|SetImmune true)
    (Variables|Default|SetPirateHealth (- (Variables|Default|GetPirateHealth) Damage))
    (Effects|SpawnEmitteratLocation "/Game/StarterContent/Particles/P_Explosion.P_Explosion" (Transformation|GetActorLocation))
    (Utilities|FlowControl|Delay (Variables|Default|GetImmuneTime))
    (Variables|Default|SetImmune false)
    (Development|PrintString (Utilities|String|ToString(Float) (Variables|Default|GetPirateHealth)))))

(fn ConstructionScript)