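; Pirate enemy character that fights, carries cargo and can leap onto boats, with a random Fighter flag and randomised morph-target looks.
; Its hit collider damages Player or Repairable actors during attacks, while incoming damage spawns blood and starts brief immunity.
; Cargo is box-traced, destroyed and shown as a carried mesh, then respawned when dropped.
; Tick polls health, dropping cargo on death, spawning gold coins once and disabling capsule collision.
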(event OnComponentBeginOverlap(HitCollider)
  (params (OverlappedComponent :type Primitive%20Component%20Object%20Reference) (OtherActor :type Actor%20Object%20Reference) (OtherComp :type Primitive%20Component%20Object%20Reference) (OtherBodyIndex :type Integer) (bFromSweep :type Boolean) (SweepResult :type Hit%20Result%20Structure%20%28by%20ref%29))
  ;[1 1 1] Hitting Player
  (if (Variables|Default|GetDamageAttackState)
    (if (Variables|Default|GetAttacking)
      (if (or (Actor|ActorHasTag OtherActor "Player") (Actor|ActorHasTag OtherActor "Repairable"))
        (Game|Damage|ApplyDamage OtherActor (Math|Conversions|ToFloat(Integer) (Variables|Default|GetStrength)) 0 0)))))

(event Custom|PickUpCargo
  (bind _returnvalue (Transformation|GetActorLocation))
  ;[1 1 1] PickUpCargo
  (if (not (and (Variables|Default|GetHoldingCargo) (Variables|Default|GetAtDestination)))
    (if (AI|Components|NavMovement|IsMovingonGround (Variables|Character|GetCharacterMovement))
      (Development|PrintString "CAST RAY")
      (bind (_outhit _returnvalue_2) (Collision|BoxTraceByChannel (+ _returnvalue "0,0.000000,-30.000000") (+ (+ _returnvalue (* (Math|Vector|GetForwardVector (Variables|Collision|GetCapsuleComponent)) (Variables|Default|GetCollectingReach))) "0,0,-30.000000") "30.000000,30.000000,30.000000" "0, 0, 0" "TraceTypeQuery2" false 0 "None"))
      (if _returnvalue_2
        (if (Actor|ActorHasTag (.hitactor _outhit) "Cargo")
          (Variables|Default|SetHoldingCargo true)
          (Rendering|SetVisibility (Variables|Default|GetCargo1) true false)
          (Actor|DestroyActor (.hitactor _outhit)))))))

(event Custom|DropCargo
  (bind _returnvalue (Transformation|GetActorLocation))
  (bind _capsulecomponent (Variables|Collision|GetCapsuleComponent))
  (bind _dropreach (Variables|Default|GetDropReach))
  (bind _returnvalue_2 (Math|Vector|GetForwardVector _capsulecomponent))
  (bind _returnvalue_3 (* _returnvalue_2 _dropreach))
  (bind _returnvalue_4 (+ _returnvalue _returnvalue_3))
  ;[1 1 1] DropCargo
  (if (AI|Components|NavMovement|IsMovingonGround (Variables|Character|GetCharacterMovement))
    (Development|PrintString "Dropping")
    (Rendering|SetVisibility (Variables|Default|GetCargo1) false false)
    (bind _returnvalue_5 (Game|SpawnActorfromClass "/Game/_Game/Blueprints/Cargo.Cargo_C" (Math|Transform|MakeTransform (Math|Vector|MakeVector (.x _returnvalue_4) (.y _returnvalue_4) (- (.z _returnvalue_4) 5e+01)) (Transformation|GetWorldRotation (Variables|Collision|GetCapsuleComponent)) "0.800000,0.800000,0.800000") "Undefined" 0 0))
    (Variables|/Game/_Game/Blueprints/Cargo.Cargo_C|SetOwnedByPlayer _returnvalue_5 false)
    (Variables|Default|SetHoldingCargo false)
    (Variables|Default|SetAtDestination false)))

(event Custom|JumpOnBoat
  (bind _returnvalue (Transformation|GetActorForwardVector))
  (Character|LaunchCharacter (Math|Vector|MakeVector (* (.x _returnvalue) 5e+02) (* (.y _returnvalue) 5e+02) 8e+02) false false))

(event Collision|EventActorBeginOverlap
  (params (OtherActor :type Actor%20Object%20Reference))
  ;[1 1 1] Morphkeys
)

(event Game|Damage|EventAnyDamage
  (params (Damage :type Float%20%28single-precision%29) (DamageType :type Damage%20Type%20Object%20Reference) (InstigatedBy :type Controller%20Object%20Reference) (DamageCauser :type Actor%20Object%20Reference))
  (bind _returnvalue (Math|Random|RandomFloatinRange 0.3 2.0))
  ;[1 1 1] Getting Damage
  (if (not (Variables|Default|GetImmune))
    (Variables|Default|SetImmune true)
    (Variables|Default|SetPirateHealth (- (Variables|Default|GetPirateHealth) Damage))
    (Effects|SpawnEmitteratLocation "/Game/Realistic_Starter_VFX_Pack_Vol2/Particles/Blood/P_Blood_Splat_Cone.P_Blood_Splat_Cone" (Transformation|GetActorLocation) (Math|Random|RandomRotator true) (Math|Vector|MakeVector _returnvalue _returnvalue _returnvalue))
    (Utilities|FlowControl|Delay (Variables|Default|GetImmuneTime))
    (Variables|Default|SetImmune false)
    (Development|PrintString (Utilities|String|ToString(Float) (Variables|Default|GetPirateHealth)))))

(event EventTick
  (params (DeltaSeconds :type Float%20%28single-precision%29))
  ;[1 1 1] Pirate Death
  (if (and (Variables|Default|GetHoldingCargo) (Variables|Default|GetDead))
    (CallFunction|DropCargo))
  (if (Variables|Default|GetGetsBlocked)
    (Utilities|FlowControl|Delay 0.2)
    (Variables|Default|SetGetsBlocked false))
  (bind _output_get (Variables|Default|SetDead (<= (Variables|Default|GetPirateHealth) 0.0)))
  (if _output_get
    (Utilities|FlowControl|DoOnce false
      (:Completed
        (Game|SpawnActorfromClass "/Game/_Game/Blueprints/Items/GoldCoins.GoldCoins_C" (Math|Transform|MakeTransform (Transformation|GetActorLocation) "0, 0, 0" "1.000000,1.000000,1.000000") "AdjustIfPossibleButAlwaysSpawn" 0 0)
        (Collision|SetCollisionEnabled (Variables|Collision|GetCapsuleComponent) "NoCollision")))))

(event EventBeginPlay
  (bind _mesh (Variables|Character|GetMesh))
  ;[1 1 1] Morphkeys
  (Variables|Default|SetFighter (Math|Random|RandomBool))
  (Components|SkeletalMesh|SetMorphTarget _mesh "mouth1" 1.0 true)
  (Components|SkeletalMesh|SetMorphTarget _mesh "mouth2" 1.0 true)
  (Components|SkeletalMesh|SetMorphTarget (Variables|Character|GetMesh) "strong" (Math|Random|RandomFloatinRange -1.0 1.0) true)
  (Components|SkeletalMesh|SetMorphTarget (Variables|Character|GetMesh) "strong" (Math|Random|RandomFloatinRange -1.0 1.0) true)
  (Components|SkeletalMesh|SetMorphTarget (Variables|Character|GetMesh) "fat" (Math|Random|RandomFloatinRange -1.0 1.0) true)
  (Components|SkeletalMesh|SetMorphTarget (Variables|Character|GetMesh) "wideface" (Math|Random|RandomFloatinRange -1.0 1.0) true)
  (Components|SkeletalMesh|SetMorphTarget (Variables|Character|GetMesh) "eyes" (Math|Random|RandomFloatinRange -1.0 1.0) true)
  (Components|SkeletalMesh|SetMorphTarget (Variables|Character|GetMesh) "cheeks" (Math|Random|RandomFloatinRange -1.0 1.0) true)
  (Components|SkeletalMesh|SetMorphTarget (Variables|Character|GetMesh) "eyes" (Math|Random|RandomFloatinRange -1.0 1.0) true)
  (Components|SkeletalMesh|SetMorphTarget (Variables|Character|GetMesh) "ears" (Math|Random|RandomFloatinRange -1.0 1.0) true)
  (Components|SkeletalMesh|SetMorphTarget (Variables|Character|GetMesh) "lowerbody" (Math|Random|RandomFloatinRange -1.0 1.0) true)
  (Components|SkeletalMesh|SetMorphTarget (Variables|Character|GetMesh) "upperbody" (Math|Random|RandomFloatinRange -1.0 1.0) true)
  (Components|SkeletalMesh|SetMorphTarget (Variables|Character|GetMesh) "longhair" (Math|Random|RandomFloatinRange -1.0 1.0) true))

(fn ConstructionScript)