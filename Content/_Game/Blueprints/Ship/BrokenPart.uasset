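; BrokenPart is a ship part actor that takes damage and destroys itself when its health runs out.
; Any damage lowers Health, prints it and spawns an explosion emitter at the actor's location, then a half-second immunity window ignores further hits.
; Tick checks Health every frame and, at zero or below, prints a break message and destroys the actor.
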(event EventBeginPlay)

(event Collision|EventActorBeginOverlap
  (params (OtherActor :type Actor%20Object%20Reference)))

(event EventTick
  (params (DeltaSeconds :type Float%20%28single-precision%29))
  (if (<= (Variables|Default|GetHealth) 0.0)
    (Development|PrintString "Part Broken!")
    (Actor|DestroyActor)))

(event Game|Damage|EventAnyDamage
  (params (Damage :type Float%20%28single-precision%29) (DamageType :type Damage%20Type%20Object%20Reference) (InstigatedBy :type Controller%20Object%20Reference) (DamageCauser :type Actor%20Object%20Reference))
  (if (not (Variables|Default|GetImmune))
    (Variables|Default|SetImmune true)
    (bind _output_get (Variables|Default|SetHealth (- (Variables|Default|GetHealth) Damage)))
    (Development|PrintString (Utilities|String|ToString(Float) _output_get))
    (Effects|SpawnEmitteratLocation "/Game/StarterContent/Particles/P_Explosion.P_Explosion" (Transformation|GetActorLocation))
    (Utilities|FlowControl|Delay 0.5)
    (Variables|Default|SetImmune false)))

(fn ConstructionScript)